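; Tank pawn for Cannon Clash that displays its health and runs a round countdown.
; Tick sets the health bar widget's percent from the Health component, assuming a maximum of 100.
; The same Tick chain uses a one-second Delay to throttle RoundTimer decrements, so the countdown depends on the widget cast succeeding.
; BeginPlay adds a countdown timer widget to the viewport, with no value passed to it here.
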(event EventBeginPlay
  (bind _returnvalue (UserInterface|CreateWidget "/Game/CannonClash/Blueprints/Widgets/WB_CountdownTimer.WB_CountdownTimer_C"))
  (UserInterface|Viewport|AddtoViewport _returnvalue 0))

(event EventTick
  (params (DeltaSeconds :type Float%20%28single-precision%29))
  (bind _aswb_tank_health_bar (Utilities|Casting|CastToWB_TankHealthBar (UserInterface|GetWidget (Variables|Default|GetHealthBarWidget))))
  (Progress|SetPercent (Variables|/Game/CannonClash/Blueprints/Widgets/WB_TankHealthBar.WB_TankHealthBar_C|GetHealthBar _aswb_tank_health_bar) (/ (Variables|/Script/CannonClash.HealthComponent|GetCurrentHealth (Variables|Default|GetHealth)) 1e+02))
  (Utilities|FlowControl|Delay 1.0)
  (Variables|Default|SetRoundTimer (- (Variables|Default|GetRoundTimer) 1)))

(fn ConstructionScript)